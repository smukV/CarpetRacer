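; Player controller for the toy vehicle that steers the controlled pawn toward the point under the cursor.
; Adds the IMC_ToyVehicle mapping context on BeginPlay; the click action traces the Visibility channel and, on a hit, feeds movement input toward that location.
; GetSpeedScale is meant to scale input by cursor distance, but its curve lookup is unconnected.
; MoveTo, a navigation move with cursor effect, is never called here.
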(event Input|EnhancedActionEvents|EnhancedInputActionIA_SetDestination_Click
  (params (ActionValue :type Boolean) (ElapsedSeconds :type Float%20%28double-precision%29) (TriggeredSeconds :type Float%20%28double-precision%29) (InputAction :type Input%20Action%20Object%20Reference :default "/Game/ToyVehicle/Input/Actions/IA_SetDestination_Click.IA_SetDestination_Click"))
  (bind (_hit _location) (CallFunction|GetLocationUnderCursor))
  (if _hit
    (CallFunction|Follow _location (Utilities|GetSpeedScale _location))))

(event EventBeginPlay
  (bind _returnvalue (PlayerController|LocalPlayerSubsystems|GetEnhancedInputLocalPlayerSubsystem))
  ;[0.05098 0.05098 0.05098] Add Mapping Context
  (Utilities|IsValid _returnvalue
    (:Is%20Valid
      (Input|AddMappingContext _returnvalue "/Game/ToyVehicle/Input/IMC_ToyVehicle.IMC_ToyVehicle" 0 "(bIgnoreAllPressedKeysUntilRelease=True,bForceImmediately=False,bNotifyUserSettings=False)"))))

(fn ConstructionScript)

(fn Moveto
  (params (Location :type Vector))
  (AI|Navigation|SimpleMovetoLocation self Location)
  (Niagara|SpawnSystematLocation (Variables|Input|GetFXCursor) Location))

(fn Follow
  (params (Location :type Vector) (Speed%20Scale :type Float%20%28single-precision%29))
  (bind _returnvalue (Pawn|GetControlledPawn))
  (Pawn|Input|AddMovementInput _returnvalue (Math|Vector|GetUnitDirection(Vector) (Transformation|GetActorLocation _returnvalue) Location) Speed%20Scale false))

(fn GetLocationUnderCursor
  (bind _hitresult (Game|Player|GetHitResultUnderCursorbyChannel "TraceTypeQuery1" true))
  (bind (_bblockinghit _binitialoverlap _time _distance _location) (Collision|BreakHitResult _hitresult))
  (return _bblockinghit _location))