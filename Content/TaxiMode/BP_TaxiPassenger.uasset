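; Taxi passenger actor for taxi mode that glows and signals when a toy vehicle arrives to pick it up.
; An overlap on the PickupZone that passes the BP_ToyVehicle class cast calls the GetInTheCar dispatcher.
; On BeginPlay it creates a dynamic material for the mesh, and a timeline drives its Emissive parameter.
; The timeline's Finished output feeds a FlipFlop that alternates play and reverse, producing a continuous pulse.
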(event OnComponentBeginOverlap(PickupZone)
  (params (OverlappedComponent :type Primitive%20Component%20Object%20Reference) (OtherActor :type Actor%20Object%20Reference) (OtherComp :type Primitive%20Component%20Object%20Reference) (OtherBodyIndex :type Integer) (bFromSweep :type Boolean) (SweepResult :type Hit%20Result%20Structure%20%28by%20ref%29))
  (Utilities|Casting|CastToBP_ToyVehicleClass (Utilities|GetClass OtherActor))
  (Default|CallGetintheCar))

(event EventBeginPlay
  (bind _returnvalue (Rendering|Material|CreateDynamicMaterialInstance (Rendering|Material|GetMaterial (Variables|Default|GetStaticMesh1) 0) "None" "None" :!class /Script/Engine.KismetMaterialLibrary))
  (bind _output_get (Variables|Default|SetDynamicMaterialReference _returnvalue))
  (Rendering|Material|SetMaterial (Variables|Default|GetStaticMesh1) 0 _output_get)
  (Utilities|FlowControl|FlipFlop :!label _label
    (:A
      (bind _glowing (Timeline|Timeline Play)
        (:Update
          (Rendering|Material|SetScalarParameterValue (Variables|Default|GetDynamicMaterialReference) "Emissive" _glowing :!class /Script/Engine.MaterialInstanceDynamic))
        (:Finished
          (goto _label))))
    (:B
      (Timeline|Timeline Reverse))))

(fn ConstructionScript)