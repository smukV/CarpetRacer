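; Decal actor that draws a road surface with lane divider lines, sized from length, road width and lane count.
; The construction script calls UpdateMaterial, which scales the main decal over all lanes and gives it a colored dynamic material.
; It then adds one fewer line decals than lanes, spaced sideways by road width, with white line materials whose sector count follows the length.
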(event EventBeginPlay)

(fn ConstructionScript
  (CallFunction|UpdateMaterial))

(fn UpdateMaterial
  (bind _lines (Variables|Default|GetLines))
  (bind _decal (Variables|Default|GetDecal))
  (bind _decal_2 (Variables|Default|GetDecal))
  (bind _returnvalue (- _lines 1))
  (bind _decalsize (Variables|/Script/Engine.DecalComponent|GetDecalSize _decal))
  (bind _decalsize_2 (Variables|/Script/Engine.DecalComponent|GetDecalSize _decal_2))
  (Utilities|FlowControl|Sequence
    (:then_0
      (Transformation|SetRelativeScale3D (Variables|Default|GetDecal) (Math|Vector|MakeVector 1.0 (/ (/ (Variables|Default|GetLength) 2.0) (.y _decalsize_2)) (/ (/ (* (Variables|Default|GetRoadWidth) (Variables|Default|GetLines)) 2.0) (.z _decalsize_2))))
      (bind _returnvalue_2 (Rendering|Material|CreateDynamicMaterialInstance "/Game/Decals/M_Decal_Color.M_Decal_Color" "None" "None" :!class /Script/Engine.KismetMaterialLibrary))
      (bind _output_get (Variables|Default|SetMaterial _returnvalue_2))
      (Rendering|Material|SetVectorParameterValue _output_get "Color" (Math|Conversions|ToLinearColor(Color) (Variables|Default|GetColor)) :!class /Script/Engine.MaterialInstanceDynamic)
      (Rendering|Components|Decal|SetDecalMaterial (Variables|Default|GetDecal) (Variables|Default|GetMaterial)))
    (:then_1
      (for _index (range 1 _returnvalue)
        (bind _returnvalue_3 (AddComponent|AddDecalComponent false))
        (Transformation|AddWorldOffset _returnvalue_3 (Math|Vector|MakeVector 0.0 (+ (* (- _index 1) (Variables|Default|GetRoadWidth)) (* (* (Variables|Default|GetRoadWidth) (/ (- _returnvalue 1) 0.0)) -1.0)) 0.0) false true)
        (Transformation|SetRelativeScale3D _returnvalue_3 (Math|Vector|MakeVector 1.0 (/ 8.0 (.z _decalsize)) (/ (Variables|Default|GetLength) (.y _decalsize))))
        (bind _returnvalue_4 (Rendering|Material|CreateDynamicMaterialInstance "/Game/Decals/M_Decal_Line.M_Decal_Line" "None" "None" :!class /Script/Engine.KismetMaterialLibrary))
        (bind _output_get_2 (Variables|Default|SetMaterial _returnvalue_4))
        (Rendering|Material|SetVectorParameterValue _output_get_2 "Color" "(R=1.000000,G=1.000000,B=1.000000,A=1.000000)" :!class /Script/Engine.MaterialInstanceDynamic)
        (Rendering|Material|SetScalarParameterValue (Variables|Default|GetMaterial) "NumSectors" (Math|Conversions|ToFloat(Integer) (Math|Float|Floor (/ (Variables|Default|GetLength) 31.4))) :!class /Script/Engine.MaterialInstanceDynamic)
        (Rendering|Components|Decal|SetDecalMaterial _returnvalue_3 (Variables|Default|GetMaterial))))))