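; BP_CircleRoad is a decal actor that draws a circular road, or a sector of one, with lane dividers.
; Its construction script calls UpdateMaterial, which scales the main decal to OuterRadius and sets color, band width and sector on a dynamic M_Decal_Circle instance.
; It then adds a thin white decal ring per boundary between lines, spaced by RoadWidth, with segment count scaled to radius.
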(event EventBeginPlay)

(fn ConstructionScript
  (CallFunction|UpdateMaterial))

(fn UpdateMaterial
  (bind _decal (Variables|Default|GetDecal))
  (Utilities|FlowControl|Sequence
    (:then_0
      (Transformation|SetRelativeScale3D (Variables|Default|GetDecal) (Math|Conversions|ToVector(Float) (/ (Variables|Default|GetOuterRadius) (.y (Variables|/Script/Engine.DecalComponent|GetDecalSize (Variables|Default|GetDecal))))))
      (bind _returnvalue (Rendering|Material|CreateDynamicMaterialInstance "/Game/Decals/M_Decal_Circle.M_Decal_Circle" "None" "None" :!class /Script/Engine.KismetMaterialLibrary))
      (bind _output_get (Variables|Default|SetMaterial _returnvalue))
      (Rendering|Material|SetVectorParameterValue _output_get "Color" (Math|Conversions|ToLinearColor(Color) (Variables|Default|GetColor)) :!class /Script/Engine.MaterialInstanceDynamic)
      (Rendering|Material|SetScalarParameterValue (Variables|Default|GetMaterial) "Width" (/ (/ (* (/ (Variables|Default|GetRoadWidth) 2.0) (Variables|Default|GetLines)) (.y (Variables|/Script/Engine.DecalComponent|GetDecalSize _decal))) (.y (Variables|/Script/Engine.SceneComponent|GetRelativeScale3D _decal))) :!class /Script/Engine.MaterialInstanceDynamic)
      (Rendering|Material|SetScalarParameterValue (Variables|Default|GetMaterial) "Sector" (Variables|Default|GetSector) :!class /Script/Engine.MaterialInstanceDynamic)
      (Rendering|Components|Decal|SetDecalMaterial (Variables|Default|GetDecal) (Variables|Default|GetMaterial)))
    (:then_1
      (for _index (range 1 (- (Variables|Default|GetLines) 1))
        (LocalVariables|SetCurrentRadius (- (+ (Variables|Default|GetOuterRadius) 2.0) (* (Variables|Default|GetRoadWidth) _index)))
        (bind _returnvalue_2 (AddComponent|AddDecalComponent false))
        (Transformation|SetRelativeScale3D _returnvalue_2 (Math|Conversions|ToVector(Float) (/ (LocalVariables|GetCurrentRadius) (.y (Variables|/Script/Engine.DecalComponent|GetDecalSize _returnvalue_2)))))
        (bind _returnvalue_3 (Rendering|Material|CreateDynamicMaterialInstance "/Game/Decals/M_Decal_Circle.M_Decal_Circle" "None" "None" :!class /Script/Engine.KismetMaterialLibrary))
        (bind _output_get_2 (Variables|Default|SetMaterial _returnvalue_3))
        (Rendering|Material|SetVectorParameterValue _output_get_2 "Color" "(R=1.000000,G=1.000000,B=1.000000,A=1.000000)" :!class /Script/Engine.MaterialInstanceDynamic)
        (Rendering|Material|SetScalarParameterValue (Variables|Default|GetMaterial) "Sector" (Variables|Default|GetSector) :!class /Script/Engine.MaterialInstanceDynamic)
        (Rendering|Material|SetScalarParameterValue (Variables|Default|GetMaterial) "NumSectors" (Math|Conversions|ToFloat(Integer) (Math|Float|Floor (/ (LocalVariables|GetCurrentRadius) 5.0))) :!class /Script/Engine.MaterialInstanceDynamic)
        (Rendering|Material|SetScalarParameterValue (Variables|Default|GetMaterial) "Width" (/ (/ 4.0 (.y (Variables|/Script/Engine.DecalComponent|GetDecalSize _returnvalue_2))) (.y (Variables|/Script/Engine.SceneComponent|GetRelativeScale3D _returnvalue_2))) :!class /Script/Engine.MaterialInstanceDynamic)
        (Rendering|Components|Decal|SetDecalMaterial _returnvalue_2 (Variables|Default|GetMaterial))))))