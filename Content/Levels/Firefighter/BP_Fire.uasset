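; Fire actor for the Firefighter level that the player puts out before its burn countdown runs out.
; Toy vehicles still inside PutoutZone after a short delay trigger an arrival dispatcher.
; Tick shrinks the fire while the player pawn overlaps the zone, counts down a text timer, and feeds an on/off-screen indicator widget.
; Extinguishing or burning down fires its own dispatcher and removes that widget.
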(event OnComponentBeginOverlap(PutoutZone)
  (params (OverlappedComponent :type Primitive%20Component%20Object%20Reference) (OtherActor :type Actor%20Object%20Reference) (OtherComp :type Primitive%20Component%20Object%20Reference) (OtherBodyIndex :type Integer) (bFromSweep :type Boolean) (SweepResult :type Hit%20Result%20Structure%20%28by%20ref%29))
  (Utilities|Casting|CastToBP_ToyVehicle OtherActor)
  (Utilities|FlowControl|Delay 0.2)
  (if (Collision|IsOverlappingActor (Variables|Default|GetPutoutZone) OtherActor :!class /Script/Engine.PrimitiveComponent)
    (Default|CallArrivedatFire (Variables|Parametres|GetTimeToExtinguish) self)))

(event EventTick
  (params (DeltaSeconds :type Float%20%28single-precision%29))
  (Utilities|FlowControl|Sequence
    (:then_0
      (if (Collision|IsOverlappingActor (Variables|Default|GetPutoutZone) (Game|Player|GetPlayerPawn 0) :!class /Script/Engine.PrimitiveComponent)
        (Transformation|SetRelativeScale3D (Variables|Default|GetFire) (Math|Conversions|ToVector(Float) (Math|Float|Lerp 3.0 1.0 (/ (Variables|Default|GetOverlapingTime) (Variables|Parametres|GetTimeToExtinguish)))))
        (Variables|Default|SetOverlapingTime (Math|Float|Clamp(Float) (+ (Variables|Default|GetOverlapingTime) DeltaSeconds) 0.0 (Variables|Parametres|GetTimeToExtinguish)))))
    (:then_1
      (if (== (Variables|Default|GetOverlapingTime) (Variables|Parametres|GetTimeToExtinguish))
        (Default|CallFireDistinguished self)
        (Widget|RemovefromParent (stale EventBeginPlay _returnvalue) :!label _label)
        (else
          (Variables|Parametres|SetTimeToBurn (Math|Float|Clamp(Float) (- (Variables|Parametres|GetTimeToBurn) DeltaSeconds) 0.0 (Variables|Parametres|GetTimeToBurn)))
          (Rendering|Components|TextRender|SetText (Variables|Default|GetTimer) (Utilities|Text|ToText(String) (Class|KismetStringLibrary|TimeSecondstoString (Math|Float|Clamp(Float) (- (Variables|Parametres|GetTimeToBurn) DeltaSeconds) 0.0 (Variables|Parametres|GetTimeToBurn)))))
          (if (> (Variables|Parametres|GetTimeToBurn) 0.0)
            (Variables|/Game/UI/OnOffScreenIndicator.OnOffScreenIndicator_C|SetTime (stale EventBeginPlay _returnvalue) (Variables|Parametres|GetTimeToBurn))
            (Variables|/Game/UI/OnOffScreenIndicator.OnOffScreenIndicator_C|SetTargeted%20Component (stale EventBeginPlay _returnvalue) self)
            (UserInterface|Viewport|AddtoViewport (stale EventBeginPlay _returnvalue) 0)
            (else
              (Default|CallBurnedDown)
              (goto _label))))))))

(event EventBeginPlay
  (bind _returnvalue (UserInterface|CreateWidget "/Game/UI/OnOffScreenIndicator.OnOffScreenIndicator_C" (Game|GetPlayerController 0)))
  (Variables|/Game/UI/OnOffScreenIndicator.OnOffScreenIndicator_C|SetTime _returnvalue (Variables|Parametres|GetTimeToBurn))
  (Variables|/Game/UI/OnOffScreenIndicator.OnOffScreenIndicator_C|SetTargeted%20Component _returnvalue self)
  (UserInterface|Viewport|AddtoViewport _returnvalue 0))

(fn ConstructionScript)